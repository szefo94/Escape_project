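; Openable door actor that swings open and closed when its OpenDoor1 component fires open or close events.
; It stores its starting rotation on BeginPlay, then the DoorSwing timeline applies a yaw offset on top of that rotation.
; A timeline event track plays the door lock sound at the actor's location, and closing simply reverses the same timeline.
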(event `self.ReceiveBeginPlay`
  (set `self.Initial Rotation` (`self.K2_GetActorRotation`)))

(event `self.OpenDoor1.OnOpen`
  (bind (_direction _open_angle) (`Timeline|Door Swing` :!label _label)
    (:`Update`
      (`self.K2_SetActorRotation` (`KismetMathLibrary.ComposeRotators` (`KismetMathLibrary.MakeRotator` 0.0 0.0 _open_angle) (`self.Initial Rotation`))))
    (:`Sound Timing`
      (`GameplayStatics.PlaySoundAtLocation` "/Game/Audio/door-lock.door-lock" (`self.K2_GetActorLocation`)))))

(event `self.OpenDoor1.OnClose`
  (goto _label :!via `Reverse`))

(fn `UserConstructionScript`)